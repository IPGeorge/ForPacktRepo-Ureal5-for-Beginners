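; BP_Boss is the boss character, armed with a BP_Hatchet spawned at begin play and attached to its right hand socket.
; AI perception sets or clears the PlayerTarget blackboard key as a BP_Hero is sensed or lost.
; Damage only lands during certain AB_Boss animation states, switching the AnimState to a hit or death state.
; On death, the weapon and boss are destroyed after a short delay.
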(event `self.ReceiveBeginPlay`
  (bind _returnvalue (`|SpawnActorFromClass` "/Game/Pangaea/Weapons/Hatchet/BP_Hatchet.BP_Hatchet_C" (`self.GetTransform`) "AlwaysSpawn" "MultiplyWithRoot" null null))
  (bind _output_get (set `self.Weapon` _returnvalue))
  (`self.K2_AttachToComponent` _output_get (`self.Mesh`) "RightHandSocket" "SnapToTarget" "SnapToTarget" "SnapToTarget" true)
  (set `self.Health` (`self.MaxHealth`)))

(event `self.AIPerception.OnTargetPerceptionInfoUpdated`
  (params (UpdateInfo :type "ActorPerceptionUpdateInfo Structure (by ref)"))
  (bind (_targetid _target _stimulus) (break `ActorPerceptionUpdateInfo` UpdateInfo))
  (bind _returnvalue (`AIBlueprintHelperLibrary.GetBlackboard` (`AIBlueprintHelperLibrary.GetAIController` self)))
  (bind _asbp_hero (cast `/Game/Pangaea/Characters/Hero/BP_Hero` _target))
  (if (`.bSuccessfullySensed` (break `AIStimulus` _stimulus))
    (`BlackboardComponent.SetValueAsObject` _returnvalue "PlayerTarget" _asbp_hero)
    (else
      (`BlackboardComponent.ClearValue` _returnvalue "PlayerTarget"))))

(event `self.ReceiveAnyDamage`
  (params (Damage :type "Float (single-precision)") (DamageType :type "DamageType Object Reference") (InstigatedBy :type "Controller Object Reference") (DamageCauser :type "Actor Object Reference"))
  (bind _asab_boss (cast `/Game/Pangaea/Characters/Boss/AB_Boss` (`SkeletalMeshComponent.GetAnimInstance` (`self.Mesh`))))
  (bind _animstate (`/Game/Pangaea/Characters/Boss/AB_Boss.AnimState` _asab_boss))
  (if (or (or (== _animstate 0) (== _animstate 11)) (== _animstate 12))
    (bind _output_get (set `self.Health` (- (`self.Health`) Damage)))
    (if (> _output_get 0.0)
      (set `/Game/Pangaea/Characters/Boss/AB_Boss.AnimState` 2 _asab_boss)
      (else
        (set `/Game/Pangaea/Characters/Boss/AB_Boss.AnimState` 3 _asab_boss)
        (`KismetSystemLibrary.Delay` 5.0)
        (`self.K2_DestroyActor` (`self.Weapon`))
        (`self.K2_DestroyActor`)))))

(fn `GetAnimInst`
  (returns (AnimInst :type "/Game/Pangaea/Characters/Boss/AB_Boss Object Reference"))
  (bind _asab_boss (cast `/Game/Pangaea/Characters/Boss/AB_Boss` (`SkeletalMeshComponent.GetAnimInstance` (`self.Mesh`))))
  (return _asab_boss))

(fn `UserConstructionScript`)