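; BP_Mission is a mission actor that prints its goal at BeginPlay and tracks whether its list of objectives is completed.
; Each Tick scans Objectives in order, activating the first incomplete one and breaking out of the loop through a custom event, so objectives run sequentially.
; Once none remain incomplete, a DoOnce shows the HUD win/lose display as a win, waits, then opens the MainMenu level.
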(event `self.ReceiveBeginPlay`
  (`KismetSystemLibrary.PrintString` (`KismetStringLibrary.Concat_StrStr` "Mission: " (`self.Goal`)) true true (struct :`G` 0.66 :`B` 1.0 :`A` 1.0) 15.0))

(event `self.ReceiveTick`
  (params (DeltaSeconds :type "Float (single-precision)"))
  (if (`self.IsCompleted`)
    ; When the mission is completed, display "You WIn!", delay and navigate to the main menu
    (`/Engine/EditorBlueprintResources/StandardMacros.DoOnce` false
      (:`Completed`
        (bind _foundwidgets (`WidgetBlueprintLibrary.GetAllWidgetsOfClass` "/Game/Pangaea/UI/HUD.HUD_C"))
        (`/Game/Pangaea/UI/HUD.ShowWinLose` (`|GetArrayItem` _foundwidgets) true)
        (`KismetSystemLibrary.Delay` 10.0)
        (`GameplayStatics.OpenLevel` "MainMenu")))
    (else
      ; For each objective, when an incomplete objective is found, activate it and set IsCompleted false
      (set `self.IsCompleted` true)
      (for _array_element (`self.Objectives`) :!label _label
        (if (not (`/Game/Pangaea/Mission/BP_Objective.IsCompleted` _array_element))
          (set `/Game/Pangaea/Mission/BP_Objective.IsActive` true _array_element)
          (set `self.IsCompleted` false)
          (`self.CustomEvent_Break`))))))

(event `CustomEvent_Break`
  ; For each objective, when an incomplete objective is found, activate it and set IsCompleted false
  (goto _label :!via `Break`))

(fn `UserConstructionScript`)